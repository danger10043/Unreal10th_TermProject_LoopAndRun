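; Color-coded switchable wall that toggles between a hidden, passable state and a solid blocking one, starting disabled.
; BeginPlay creates dynamic material instances for three slots on the base and outline meshes, tinting them and the Niagara effect with Color.
; Overlap events track players inside the actor.
; EnableBlock shows the base mesh, enables box collision, activates Niagara and defeats tracked players, while DisableBlock hides the mesh and removes collision.
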(event EventBeginPlay
  (bind _meshbase (Variables|Default|GetMeshBase))
  (bind _meshbase_2 (Variables|Default|GetMeshBase))
  (bind _meshoutline (Variables|Default|GetMeshOutline))
  (bind _meshoutline_2 (Variables|Default|GetMeshOutline))
  (bind _meshoutline_3 (Variables|Default|GetMeshOutline))
  (bind _meshbase_3 (Variables|Default|GetMeshBase))
  (Variables|Default|SetbIsBlocking false)
  (Utilities|FlowControl|Sequence
    (:then_0
      (bind _returnvalue (Rendering|Material|CreateDynamicMaterialInstance _meshbase_2 0 (Rendering|Material|GetMaterial _meshbase_2 0) "None" :!class /Script/Engine.PrimitiveComponent))
      (Utilities|Array|SetArrayElem (Variables|Default|GetMeshBaseColorMIDList) 0 _returnvalue)
      (bind _returnvalue_2 (Rendering|Material|CreateDynamicMaterialInstance _meshoutline_2 0 (Rendering|Material|GetMaterial _meshoutline_2 0) "None" :!class /Script/Engine.PrimitiveComponent))
      (Utilities|Array|SetArrayElem (Variables|Default|GetMeshOutlineColorMIDList) 0 _returnvalue_2)
      (Rendering|Material|SetVectorParameterValue (Utilities|Array|Get(acopy) (Variables|Default|GetMeshOutlineColorMIDList)) "Color" (Variables|Default|GetColor) :!class /Script/Engine.MaterialInstanceDynamic)
      (Rendering|Material|SetVectorParameterValue (Utilities|Array|Get(acopy) (Variables|Default|GetMeshBaseColorMIDList)) "Color" (Variables|Default|GetColor) :!class /Script/Engine.MaterialInstanceDynamic))
    (:then_1
      (bind _returnvalue_3 (Rendering|Material|CreateDynamicMaterialInstance _meshbase_3 1 (Rendering|Material|GetMaterial _meshbase_3 1) "None" :!class /Script/Engine.PrimitiveComponent))
      (Utilities|Array|SetArrayElem (Variables|Default|GetMeshBaseColorMIDList) 1 _returnvalue_3)
      (bind _returnvalue_4 (Rendering|Material|CreateDynamicMaterialInstance _meshoutline_3 1 (Rendering|Material|GetMaterial _meshoutline_3 1) "None" :!class /Script/Engine.PrimitiveComponent))
      (Utilities|Array|SetArrayElem (Variables|Default|GetMeshOutlineColorMIDList) 1 _returnvalue_4)
      (Rendering|Material|SetVectorParameterValue (Utilities|Array|Get(acopy) (Variables|Default|GetMeshOutlineColorMIDList) 1) "Color" (Variables|Default|GetColor) :!class /Script/Engine.MaterialInstanceDynamic)
      (Rendering|Material|SetVectorParameterValue (Utilities|Array|Get(acopy) (Variables|Default|GetMeshBaseColorMIDList) 1) "SphereColor" (Variables|Default|GetColor) :!class /Script/Engine.MaterialInstanceDynamic))
    (:then_2
      (bind _returnvalue_5 (Rendering|Material|CreateDynamicMaterialInstance _meshbase 2 (Rendering|Material|GetMaterial _meshbase 2) "None" :!class /Script/Engine.PrimitiveComponent))
      (Utilities|Array|SetArrayElem (Variables|Default|GetMeshBaseColorMIDList) 2 _returnvalue_5)
      (bind _returnvalue_6 (Rendering|Material|CreateDynamicMaterialInstance _meshoutline 2 (Rendering|Material|GetMaterial _meshoutline 2) "None" :!class /Script/Engine.PrimitiveComponent))
      (Utilities|Array|SetArrayElem (Variables|Default|GetMeshOutlineColorMIDList) 2 _returnvalue_6)
      (Rendering|Material|SetVectorParameterValue (Utilities|Array|Get(acopy) (Variables|Default|GetMeshOutlineColorMIDList) 2) "Color" (Variables|Default|GetColor) :!class /Script/Engine.MaterialInstanceDynamic)
      (Rendering|Material|SetVectorParameterValue (Utilities|Array|Get(acopy) (Variables|Default|GetMeshBaseColorMIDList) 2) "Color" (Variables|Default|GetColor) :!class /Script/Engine.MaterialInstanceDynamic)
      (CallFunction|DisableBlock)
      (Niagara|SetNiagaraVariable(LinearColor) (Variables|Default|GetNiagara) "User.UserColor" (Variables|Default|GetColor)))))

(event Collision|EventActorBeginOverlap
  (params (OtherActor :type Actor%20Object%20Reference))
  (bind _asbp_base_player (Utilities|Casting|CastToBP_BasePlayer OtherActor))
  (Utilities|Set|Add (Variables|Default|GetInPlayerList) _asbp_base_player))

(event Collision|EventActorEndOverlap
  (params (OtherActor :type Actor%20Object%20Reference))
  (bind _asbp_base_player (Utilities|Casting|CastToBP_BasePlayer OtherActor))
  (Utilities|Set|Remove (Variables|Default|GetInPlayerList) _asbp_base_player))

(fn ConstructionScript)

(fn EnableBlock
  (Development|SetHiddeninGame (Variables|Default|GetMeshBase) false false)
  (Collision|SetCollisionEnabled (Variables|Default|GetBoxCollision) "QueryAndPhysics")
  (Variables|Default|SetbIsBlocking true)
  (Components|Activation|Activate (Variables|Default|GetNiagara) false)
  (bind _valuepin (Utilities|Set|ForEachLoop(Set) (Variables|Default|GetInPlayerList))
    (:then
      (Default|Defeat _valuepin))
    (:CompletedPin
      (return))))

(fn DisableBlock
  (Development|SetHiddeninGame (Variables|Default|GetMeshBase) true false)
  (Collision|SetCollisionEnabled (Variables|Default|GetBoxCollision) "NoCollision")
  (Variables|Default|SetbIsBlocking false)
  (return))