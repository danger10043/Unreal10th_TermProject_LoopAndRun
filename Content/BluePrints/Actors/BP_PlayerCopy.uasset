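; BP_PlayerCopy is a player copy that replays input recorded in the game state's input list.
; TickOverride calls ApplyState, which applies at most one due entry per call, timed relative to the pawn's creation tick, to left, right and jump flags.
; Move turns those flags into swept world offsets, jumping only when grounded.
; Goal spawns a Niagara effect, then hides the copy and disables its collision and tick.
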(event EventBeginPlay
  (|CallParentFunction) ; 지금 이 노드는 비활성 상태입니다. \n핀을 끌어서 다른 노드를 연결하면 활성화됩니다.
)

(event EventTick
  (params (DeltaSeconds :type Float%20%28single-precision%29))
  (|CallParentFunction DeltaSeconds) ; 지금 이 노드는 비활성 상태입니다. \n핀을 끌어서 다른 노드를 연결하면 활성화됩니다.
)

(event Collision|EventActorBeginOverlap
  (params (OtherActor :type Actor%20Object%20Reference)))

(fn ConstructionScript
  (|CallParentFunction))

(fn ApplyState
  (bind _currentinputdatalistindex (Variables|Default|GetCurrentInputDataListIndex))
  (bind _currentgamestate (Variables|Default|GetCurrentGameState))
  (bind _inputdatalist (Variables|/Game/BluePrints/FrameWorks/GS_LevelState.GS_LevelState_C|GetInputDataList _currentgamestate))
  (bind _output (Utilities|Array|Get(acopy) _inputdatalist _currentinputdatalistindex))
  (bind (_inputdata _ispressed _executetick) (Utilities|Struct|BreakF_InputData _output))
  (if (< (Variables|Default|GetCurrentInputDataListIndex) (Utilities|Array|Length _inputdatalist))
    (if (>= (- (Variables|/Game/BluePrints/FrameWorks/GS_LevelState.GS_LevelState_C|GetCurrentTick (Variables|Default|GetCurrentGameState)) (Variables|Default|GetWorldTickThisPawnCreated)) _executetick)
      (switch Utilities|FlowControl|Switch|SwitchonE_InputDataEnum _inputdata
        (:NewEnumerator0
          (Variables|Default|SetKey_Left _ispressed))
        (:NewEnumerator1
          (Variables|Default|SetKey_Right _ispressed))
        (:NewEnumerator2
          (Variables|Default|SetKey_Jump _ispressed)))
      (Math|Integer|IncrementInt (Variables|Default|GetCurrentInputDataListIndex)
        (:%20%20
          (return))))))

(fn Goal
  (bind _returnvalue (Transformation|GetActorLocation))
  (Niagara|SpawnSystematLocation "/Game/BluePrints/VFX/NS_PlayerGoal.NS_PlayerGoal" (Math|Vector|MakeVector (.x _returnvalue) (.y _returnvalue) (- (.z _returnvalue) 4e+01)) "0, 0, 0" "0.500000,0.500000,1.000000")
  (Rendering|SetActorHiddenInGame true)
  (Collision|SetActorEnableCollision false)
  (Actor|Tick|SetActorTickEnabled false)
  (|CallParentFunction))

(fn TickOverride
  (CallFunction|ApplyState)
  (CallFunction|Move)
  (|CallParentFunction))

(fn Move
  (Variables|Default|SetDirection "0, 0, 0")
  (if (Variables|Default|GetKey_Left)
    (Variables|Default|SetDirection (+ (Variables|Default|GetDirection) (Math|Vector|MakeVector -1.0 0.0 0.0))))
  (if (Variables|Default|GetKey_Right)
    (bind _output_get (Variables|Default|SetDirection (+ (Variables|Default|GetDirection) (Math|Vector|MakeVector 1.0 0.0 0.0)))))
  (Transformation|AddActorWorldOffset (* _output_get (Variables|Default|GetSpeed)) true)
  (if (and (Variables|Default|GetKey_Jump) (Variables|Default|GetbIsGround))
    (bind _output_get_2 (Variables|Default|SetZVelocity (Variables|Default|GetJumpHeight)))
    (Transformation|AddActorWorldOffset (Math|Vector|MakeVector 0.0 0.0 (Math|Conversions|ToFloat(Integer) _output_get_2)) true)
    (|CallParentFunction)))