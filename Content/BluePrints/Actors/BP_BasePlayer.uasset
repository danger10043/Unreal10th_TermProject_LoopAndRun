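; Base player actor shared by the Player and Copy characters, which customize it through empty overrides such as Initialize, Move, Goal and TickOverride.
; Each tick derives velocity from position change, faces the movement direction, counts input-idle ticks and applies hand-rolled gravity with swept offsets for ground detection.
; Handles super jumps, orb pickup that ignores orb walls and reveals a pulsing leader-pose outline mesh, and an unstable state that defeats both players on contact.
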(event Custom|Test%20Custom
  (Development|PrintString "디버그 이벤트 실행")
  (CallFunction|SetUnstable))

(event EventBeginPlay
  (bind _skeletaloutlinemesh (Variables|Default|GetSkeletalOutlineMesh))
  ;[0.15 0.15 0.15 0.5] Player와 Copy가 공유하는 변수를 선언하고, 각자가 따로 사용하는 내용은 Initialize() 오버라이드하여 사용
  (bind _asgs_test_level_state (Utilities|Casting|CastToGS_TestLevelState (Game|GetGameState)))
  (bind _output_get (Variables|Default|SetCurrentGameState _asgs_test_level_state))
  (Variables|Default|SetWorldTickThisPawnCreated (Variables|/Game/BluePrints/FrameWorks/GS_TestLevelState.GS_TestLevelState_C|GetCurrentTick _output_get))
  (Development|SetHiddeninGame _skeletaloutlinemesh true false)
  (bind _returnvalue (Rendering|Material|CreateDynamicMaterialInstance (Variables|Default|GetSkeletalOutlineMesh) 0 (Rendering|Material|GetMaterial _skeletaloutlinemesh 0) "None" :!class /Script/Engine.PrimitiveComponent))
  (Variables|Default|SetSkeletalOutlineColorMID _returnvalue)
  (Components|SkinnedMesh|SetLeaderPoseComponent (Variables|Default|GetSkeletalOutlineMesh) (Variables|Default|GetSkeletalMesh) false false)
  (CallFunction|Initialize)
  (bind _outline_tickness_alpha (Timeline|Outline%20Tickness Play)
    (:Update
      (Rendering|Material|SetScalarParameterValue (Variables|Default|GetSkeletalOutlineColorMID) "Tickness" (* _outline_tickness_alpha 6.0) :!class /Script/Engine.MaterialInstanceDynamic))))

(event Collision|EventHit
  (params (MyComp :type Primitive%20Component%20Object%20Reference) (Other :type Actor%20Object%20Reference) (OtherComp :type Primitive%20Component%20Object%20Reference) (bSelfMoved :type Boolean) (HitLocation :type Vector :default "0, 0, 0") (HitNormal :type Vector :default "0, 0, 0") (NormalImpulse :type Vector :default "0, 0, 0") (Hit :type Hit%20Result%20Structure%20%28by%20ref%29))
  (bind _asbp_base_player (Utilities|Casting|CastToBP_BasePlayer Other))
  (if (Variables|BP_BasePlayer_C|GetbIsUnstable _asbp_base_player)
    (CallFunction|Defeat _asbp_base_player)
    (CallFunction|Defeat)))

(event EventTick
  (params (DeltaSeconds :type Float%20%28single-precision%29))
  (bind _current_velocity (CallFunction|CalculateVelocity))
  (CallFunction|RotateActor _current_velocity)
  (CallFunction|CalculateNoActionDuration)
  (CallFunction|ApplyGravity)
  (CallFunction|TickOverride))

(fn ConstructionScript)

(fn Initialize
  (return))

(fn Move
  (return))

(fn SetHasOrb
  ;[0.15 0.15 0.15 0.5] 보라색 환영 구체를 얻은 경우, 보라색 환영 벽의 충돌은 모두 무시한다.
  (Variables|Default|SetbHasOrb true)
  (for _array_element (Variables|/Game/BluePrints/FrameWorks/GS_TestLevelState.GS_TestLevelState_C|GetOrbWallList (Variables|Default|GetCurrentGameState))
    (Collision|IgnoreActorwhenMoving (Variables|Default|GetBoxCollision) _array_element true))
  (Development|SetHiddeninGame (Variables|Default|GetSkeletalOutlineMesh) false false)
  (return))

(fn SetUnstable
  (Variables|Default|SetbIsUnstable true)
  (Niagara|SpawnSystemAttached "/Game/BluePrints/VFX/NS_PlayerUnstableMode.NS_PlayerUnstableMode" (Variables|Default|GetNiagara) "None" "0, 0, 0" "0, 0, 0" "KeepRelativeOffset" false)
  (return))

(fn Goal
  (return))

(fn SuperJump
  (params (Jump%20Height :type Integer))
  ;[0.15 0.15 0.15 0.5] 슈퍼 점프 발판을 밟은 경우 Z 방향 속도 증가.
  (Variables|Default|SetZVelocity Jump%20Height)
  (return))

(fn Defeat
  ;[0.15 0.15 0.15 0.5] 피해를 주는 액터에 영향을 받았을 때, 게임 내에서 제거하는 함수.
  (Niagara|SpawnSystematLocation "/Game/BluePrints/VFX/NS_PlayerDefeat.NS_PlayerDefeat" (Transformation|GetActorLocation) "0, 0, 0" "0.700000,0.700000,0.700000")
  (Input|DisableInput 0)
  (Rendering|SetActorHiddenInGame true)
  (Collision|SetActorEnableCollision false)
  (Actor|Tick|SetActorTickEnabled false)
  (return))

(fn ApplyGravity
  ;[0.15 0.15 0.15 0.5] 중력 구현
  (bind _output_get (Variables|Default|SetZVelocity (- (Variables|Default|GetZVelocity) (Variables|Default|GetGravity))))
  (bind _sweephitresult (Transformation|AddActorWorldOffset (Math|Vector|MakeVector 0.0 0.0 (Math|Conversions|ToFloat(Integer) _output_get)) true))
  ;[0.15 0.15 0.15 0.5] 지면 충돌 시 점프 가능 여부 및 Z 방향 속도 설정
  (if (.bBlockingHit (Collision|BreakHitResult _sweephitresult))
    (if (<= (Variables|Default|GetZVelocity) 0)
      (Variables|Default|SetbIsGround true)
      (else
        (Variables|Default|SetbIsGround false)))
    (Variables|Default|SetZVelocity 0)
    (else
      (Variables|Default|SetbIsGround false)))
  (return))

(fn TickOverride
  (return))

(fn CalculateVelocity
  ;[0.15 0.15 0.15 0.5] 현재 속도를 계산하기 위한 위치 저장
  (Variables|Default|SetPreviousLocation (Variables|Default|GetCurrentLocation))
  (Variables|Default|SetCurrentLocation (Transformation|GetActorLocation))
  (bind _output_get (Variables|Default|SetCurrentVelocity (- (Variables|Default|GetCurrentLocation) (Variables|Default|GetPreviousLocation))))
  (return _output_get))

(fn RotateActor
  (params (In%20Velocity :type Vector))
  (if (> (Math|Vector|VectorLengthXY In%20Velocity) 0.0)
    (Transformation|SetActorRotation (Math|Rotator|MakeRotfromX (Class|KismetMathLibrary|VectorNormal2D In%20Velocity 0.0001))))
  (return))

(fn CalculateNoActionDuration
  (if (Math|Boolean|ORBoolean (Variables|Default|GetKey_Left) (Variables|Default|GetKey_Right) (Variables|Default|GetKey_Jump))
    (Variables|Default|SetNoActionDuration 0)
    (else
      (Math|Integer|IncrementInt (Variables|Default|GetNoActionDuration)
        (:%20%20
          _))))
  (return))

(fn TestFunction
  (Development|PrintString "디버그 함수 실행"))