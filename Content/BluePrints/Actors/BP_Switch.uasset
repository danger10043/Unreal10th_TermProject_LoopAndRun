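; Pressure switch actor that enables blocks on its TargetWalls while players overlap it and disables them when the press count drops to zero.
; Pressing plays three timelines that float, brighten and scale a star through its transform and a dynamic material, reversing them on release.
; Tick spins the active star or eases its yaw back to zero, and spawns or destroys a Niagara effect that follows it.
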(event Custom|Star%20Glow%20Disable
  (Utilities|FlowControl|Sequence
    (:then_0
      (bind _star_floating_relative_height (Timeline|Star%20Floating%20Timeline Reverse)
        (:Update
          (Transformation|SetRelativeLocation (Variables|Default|GetStar) (Math|Vector|MakeVector 0.0 -1.5e+02 _star_floating_relative_height) false false))))
    (:then_1
      (bind _star_color_alpha (Timeline|Star%20Color%20Timeline Reverse)
        (:Update
          (Rendering|Material|SetVectorParameterValue (Variables|Default|GetStarColorMID) "Color" (Math|Color|Lerp(LinearColor) (Variables|Default|GetDarkStarColor) (Variables|Default|GetStarColor) _star_color_alpha) :!class /Script/Engine.MaterialInstanceDynamic))))
    (:then_2
      (bind _star_color_alpha_2 (Timeline|Star%20Scale%20Timeline Reverse)
        (:Update
          (Transformation|SetWorldScale3D (Variables|Default|GetStar) (Math|Vector|MakeVector (Math|Float|Lerp 0.5 1.0 _star_color_alpha_2) (Math|Float|Lerp 0.5 1.0 _star_color_alpha_2) (Math|Float|Lerp 0.5 1.0 _star_color_alpha_2))))))))

(event Custom|Star%20Glow%20Enable
  (Utilities|FlowControl|Sequence
    (:then_0
      (bind _star_floating_relative_height (Timeline|Star%20Floating%20Timeline Play)
        (:Update
          (Transformation|SetRelativeLocation (Variables|Default|GetStar) (Math|Vector|MakeVector 0.0 -1.5e+02 _star_floating_relative_height) false false))))
    (:then_1
      (bind _star_color_alpha (Timeline|Star%20Color%20Timeline Play)
        (:Update
          (Rendering|Material|SetVectorParameterValue (Variables|Default|GetStarColorMID) "Color" (Math|Color|Lerp(LinearColor) (Variables|Default|GetDarkStarColor) (Variables|Default|GetStarColor) _star_color_alpha) :!class /Script/Engine.MaterialInstanceDynamic))))
    (:then_2
      (bind _star_color_alpha_2 (Timeline|Star%20Scale%20Timeline Play)
        (:Update
          (Transformation|SetWorldScale3D (Variables|Default|GetStar) (Math|Vector|MakeVector (Math|Float|Lerp 0.5 1.0 _star_color_alpha_2) (Math|Float|Lerp 0.5 1.0 _star_color_alpha_2) (Math|Float|Lerp 0.5 1.0 _star_color_alpha_2))))))))

(event EventBeginPlay
  (bind _star (Variables|Default|GetStar))
  (bind _returnvalue (Rendering|Material|CreateDynamicMaterialInstance _star 0 (Rendering|Material|GetMaterial _star 0) "None" :!class /Script/Engine.PrimitiveComponent))
  (Variables|Default|SetStarColorMID _returnvalue)
  (Variables|Default|SetDarkStarColor (* (Variables|Default|GetStarColor) "(R=0.100000,G=0.100000,B=0.100000,A=1.000000)"))
  (Rendering|Material|SetVectorParameterValue (Variables|Default|GetStarColorMID) "Color" (Variables|Default|GetDarkStarColor) :!class /Script/Engine.MaterialInstanceDynamic))

(event Collision|EventActorBeginOverlap
  (params (OtherActor :type Actor%20Object%20Reference))
  (Utilities|Casting|CastToBP_BasePlayer OtherActor)
  (if true
    (Math|Integer|IncrementInt (Variables|Default|GetPressCount)
      (:%20%20
        (CallFunction|EnableSwitch)
        (for _array_element (Variables|Default|GetTargetWalls)
          (Default|EnableBlock _array_element))))))

(event EventTick
  (params (DeltaSeconds :type Float%20%28single-precision%29))
  (CallFunction|TickStarRotate)
  (CallFunction|ApplyStarEffect))

(event Collision|EventActorEndOverlap
  (params (OtherActor :type Actor%20Object%20Reference))
  (Utilities|Casting|CastToBP_BasePlayer OtherActor)
  (if true
    (bind _result (Math|Integer|DecrementInt (Variables|Default|GetPressCount))
      (:%20%20
        (if (<= _result 0)
          (CallFunction|DisableSwitch)
          (for _array_element (Variables|Default|GetTargetWalls)
            (Default|DisableBlock _array_element)))))))

(fn ConstructionScript)

(fn EnableSwitch
  (Variables|Default|SetbIsStarEnabled true)
  (CallFunction|StarGlowEnable)
  (return))

(fn DisableSwitch
  (Variables|Default|SetbIsStarEnabled false)
  (CallFunction|StarGlowDisable)
  (return))

(fn TickStarRotate
  (bind _star (Variables|Default|GetStar))
  (bind _relativerotation (Variables|/Script/Engine.SceneComponent|GetRelativeRotation _star))
  (if (Variables|Default|GetbIsStarEnabled)
    (Transformation|AddRelativeRotation (Variables|Default|GetStar) "0.000000,7.000000,0.000000" false false)
    (return)
    (elif (> (Math|Float|Absolute(Float) (.yaw (Variables|/Script/Engine.SceneComponent|GetRelativeRotation (Variables|Default|GetStar)))) 0.0)
      (if (> (Math|Float|Absolute(Float) (.yaw _relativerotation)) 0.03)
        (Transformation|SetRelativeRotation (Variables|Default|GetStar) (Math|Rotator|MakeRotator 0.0 0.0 (* (.yaw _relativerotation) 0.9)) false false)
        (return)
        (else
          (Transformation|SetRelativeRotation (Variables|Default|GetStar) (Math|Rotator|MakeRotator 0.0 0.0 0.0) false false)
          (return)))
      (else
        (return)))))

(fn ApplyStarEffect
  (bind _star (Variables|Default|GetStar))
  (bind _relativelocation (Variables|/Script/Engine.SceneComponent|GetRelativeLocation _star))
  (Transformation|SetRelativeLocation (Variables|Default|GetStarNiagara) (Math|Vector|MakeVector (.x _relativelocation) -2e+02 (.z _relativelocation)) false false)
  (if (Variables|Default|GetbIsStarEnabled)
    (if (not (Variables|Default|GetbIsStarEffectSpawned))
      (bind _returnvalue (Niagara|SpawnSystemAttached "/Game/BluePrints/VFX/NS_SwitchEnabled.NS_SwitchEnabled" (Variables|Default|GetStarNiagara) "None" "0, 0, 0" "0, 0, 0" "KeepRelativeOffset" false))
      (Variables|Default|SetbIsStarEffectSpawned true)
      (Variables|Default|SetStarEffect _returnvalue))
    (elif (Variables|Default|GetbIsStarEffectSpawned)
      (Components|DestroyComponent (Variables|Default|GetStarEffect))
      (Variables|Default|SetbIsStarEffectSpawned false))))