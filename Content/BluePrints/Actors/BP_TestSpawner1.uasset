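; BP_TestSpawner1 is a test spawner actor that spawns an unstable BP_PlayerCopy at its own transform.
; BeginPlay creates a dynamic material instance from the Sphere's material.
; StartSpawn plays a timeline that blends that material's Color from white to yellow via an alpha track, while an event track triggers the spawn if Spawnable is true and calls SetUnstable on the new copy.
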(event Custom|Start%20Spawn
  (bind _coloralpha (Timeline|타임라인 Play)
    (:Update
      (Rendering|Material|SetVectorParameterValue (Variables|Default|GetColorMID) "Color" (Math|Color|Lerp(LinearColor) "(R=1.000000,G=1.000000,B=1.000000,A=1.000000)" "(R=1.000000,G=1.000000,B=0.000000,A=1.000000)" _coloralpha) :!class /Script/Engine.MaterialInstanceDynamic))
    (:Event%20Trigger
      (if (Variables|Default|GetbSpawnable)
        (bind _returnvalue (Game|SpawnActorfromClass "/Game/BluePrints/Actors/BP_PlayerCopy.BP_PlayerCopy_C" (Transformation|GetActorTransform) "Undefined" "MultiplyWithRoot" 0 0))
        (Default|SetUnstable _returnvalue)))))

(event EventBeginPlay
  (bind _sphere (Variables|Default|GetSphere))
  (bind _returnvalue (Rendering|Material|CreateDynamicMaterialInstance _sphere 0 (Rendering|Material|GetMaterial _sphere 0) "None" :!class /Script/Engine.PrimitiveComponent))
  (Variables|Default|SetColorMID _returnvalue))

(event EventTick
  (params (DeltaSeconds :type Float%20%28single-precision%29)))

(fn ConstructionScript)