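; BP_Orb is a spinning pickup actor that marks the player as holding an orb on overlap.
; BeginPlay spawns a glow Niagara effect slightly offset from the orb, and Tick rotates the mesh by a fixed step each frame.
; Overlap with a BP_BasePlayer calls SetHasOrb and spawns a loot pickup effect at that player's Niagara component, without hiding or destroying the orb here.
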(event EventTick
  (params (DeltaSeconds :type Float%20%28single-precision%29))
  (Transformation|AddWorldRotation (Variables|Default|GetOrbMesh) "0.000000,5.000000,0.000000" false false))

(event Collision|EventActorBeginOverlap
  (params (OtherActor :type Actor%20Object%20Reference))
  (bind _asbp_base_player (Utilities|Casting|CastToBP_BasePlayer OtherActor))
  (Default|SetHasOrb _asbp_base_player)
  (Niagara|SpawnSystematLocation "/Game/ExternalAsset/LootandPickupVFXPack/LootVFX/PickupInteraction/NS_LootPickup01.NS_LootPickup01" (Transformation|GetWorldLocation (Variables|/Game/BluePrints/Actors/BP_BasePlayer.BP_BasePlayer_C|GetNiagara _asbp_base_player))))

(event EventBeginPlay
  (bind _returnvalue (Transformation|GetActorLocation))
  (Niagara|SpawnSystematLocation "/Game/BluePrints/VFX/NS_OrbGlow.NS_OrbGlow" (Math|Vector|MakeVector (.x _returnvalue) (- (.y _returnvalue) 15.0) (.z _returnvalue))))

(fn ConstructionScript)