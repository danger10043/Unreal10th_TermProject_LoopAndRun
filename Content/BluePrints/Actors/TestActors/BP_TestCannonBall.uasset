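; BP_TestCannonBall is a test projectile actor that moves forward each frame by its Velocity, without sweep or delta-time scaling.
; On BeginPlay it records the current tick from GS_TestLevelState and destroys itself once more than TickLife game-state ticks have passed.
; On overlap with an actor implementing BPI_TestDefeat, it sends DefeatMessage to that actor and destroys itself.
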(event EventBeginPlay
  (bind _asgs_test_level_state (Utilities|Casting|CastToGS_TestLevelState (Game|GetGameState)))
  (bind _output_get (Variables|Default|SetTargetGameState _asgs_test_level_state))
  (Variables|Default|SetTickThisBulletCreated (Variables|/Game/BluePrints/FrameWorks/GS_TestLevelState.GS_TestLevelState_C|GetCurrentTick _output_get)))

(event Collision|EventActorBeginOverlap
  (params (OtherActor :type Actor%20Object%20Reference))
  (if (Utilities|DoesObjectImplementInterface OtherActor "/Game/BluePrints/FrameWorks/BPI_TestDefeat.BPI_TestDefeat_C")
    (Class|BPITestDefeat|Defeat(Message) OtherActor)
    (Actor|DestroyActor)))

(event EventTick
  (params (DeltaSeconds :type Float%20%28single-precision%29))
  (Transformation|AddActorWorldOffset (* (Transformation|GetActorForwardVector) (Variables|Default|GetVelocity)))
  (if (< (Variables|Default|GetTickLife) (- (Variables|/Game/BluePrints/FrameWorks/GS_TestLevelState.GS_TestLevelState_C|GetCurrentTick (Variables|Default|GetTargetGameState)) (Variables|Default|GetTickThisBulletCreated)))
    (Actor|DestroyActor)))

(fn ConstructionScript)