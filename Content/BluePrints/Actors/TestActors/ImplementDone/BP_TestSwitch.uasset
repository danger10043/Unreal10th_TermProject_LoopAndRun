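; BP_TestSwitch is a test pressure switch that toggles blocking on its assigned TargetWalls while players stand on it.
; At BeginPlay it tints the Switch mesh to SwitchColor through a dynamic material instance.
; BP_BasePlayer overlaps increment a press count, lower the switch and call EnableBlock on each wall.
; When the last player leaves, it raises the switch and calls DisableBlock.
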(event EventBeginPlay
  (bind _switch (Variables|Default|GetSwitch))
  (bind _returnvalue (Rendering|Material|CreateDynamicMaterialInstance _switch 0 (Rendering|Material|GetMaterial _switch 0) "None" :!class /Script/Engine.PrimitiveComponent))
  (bind _output_get (Variables|Default|SetSwitchColorMID _returnvalue))
  (Rendering|Material|SetScalarParameterValue _output_get "Opacity" 1.0 :!class /Script/Engine.MaterialInstanceDynamic)
  (Rendering|Material|SetVectorParameterValue (Variables|Default|GetSwitchColorMID) "Color" (Variables|Default|GetSwitchColor) :!class /Script/Engine.MaterialInstanceDynamic))

(event Collision|EventActorBeginOverlap
  (params (OtherActor :type Actor%20Object%20Reference))
  (Utilities|Casting|CastToBP_BasePlayer OtherActor)
  (if true
    (Math|Integer|IncrementInt (Variables|Default|GetPressCount)
      (:%20%20
        (Transformation|SetRelativeLocation (Variables|Default|GetSwitch) "0.000000,0.000000,15.000000" false false)
        (for _array_element (Variables|Default|GetTargetWalls)
          (Default|EnableBlock _array_element))))))

(event Collision|EventActorEndOverlap
  (params (OtherActor :type Actor%20Object%20Reference))
  (Utilities|Casting|CastToBP_BasePlayer OtherActor)
  (if true
    (bind _result (Math|Integer|DecrementInt (Variables|Default|GetPressCount))
      (:%20%20
        (if (<= _result 0)
          (Transformation|SetRelativeLocation (Variables|Default|GetSwitch) "0.000000,0.000000,30.000000" false false)
          (for _array_element (Variables|Default|GetTargetWalls)
            (Default|DisableBlock _array_element)))))))

(fn ConstructionScript)