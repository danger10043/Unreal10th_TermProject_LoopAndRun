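; Test goal ring actor that unlocks after enough lock increments, then requires four player passes to finish the level.
; IncreaseLockCount, not called within this Blueprint, tints a dynamic material from gray toward red, then opens the ring and starts a timeline-driven float.
; Player overlaps while open call Goal on BP_BasePlayer and change the ring color per count.
; At four goals, a timeline spins the ring and NextLevelName loads after a short delay.
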(event Custom|Start%20Floating
  (bind _floatingheightalpha (Timeline|타임라인 Play)
    (:Update
      (Transformation|SetRelativeLocation (Variables|Default|GetRing) (Math|Vector|MakeVector 0.0 0.0 (* _floatingheightalpha (Variables|Default|GetFloatingHeight))) false false))))

(event Custom|Clear%20Level
  (Game|OpenLevel(byName) (Variables|Default|GetNextLevelName)))

(event Custom|Apply%20Current%20Color
  (switch int (Variables|Default|GetGoalCount)
    (:Default
      (CallFunction|ChangeColor "(R=0.000000,G=2.000000,B=3.000000,A=1.000000)" :!label _label))
    (:0
      (CallFunction|ChangeColor "(R=1.000000,G=1.000000,B=1.000000,A=1.000000)"))
    (:1
      (CallFunction|ChangeColor "(R=1.000000,G=0.000000,B=0.000000,A=1.000000)"))
    (:2
      (CallFunction|ChangeColor "(R=1.000000,G=1.000000,B=0.000000,A=1.000000)"))
    (:3
      (CallFunction|ChangeColor "(R=0.000000,G=1.000000,B=0.000000,A=1.000000)"))
    (:4
      (goto _label))))

(event Custom|Change%20Color
  (params (In%20Color :type Linear%20Color%20Structure))
  (Rendering|Material|SetVectorParameterValue (Variables|Default|GetRingColorMID) "Color" In%20Color :!class /Script/Engine.MaterialInstanceDynamic))

(event Custom|Increase%20Lock%20Count
  (bind _result (Math|Integer|IncrementInt (Variables|Default|GetLockCount))
    (:%20%20
      (if (>= _result (Variables|Default|GetMaxLockCount))
        (Variables|Default|SetbIsOpened true)
        (CallFunction|StartFloating)
        (CallFunction|ApplyCurrentColor)
        (else
          (CallFunction|ApplyLockColor))))))

(event Custom|Start%20Spinning
  (bind _rotationalpha (Timeline|타임라인_0 Play)
    (:Update
      (Transformation|AddRelativeRotation (Variables|Default|GetRing) (Math|Rotator|MakeRotator 0.0 0.0 (* _rotationalpha (Variables|Default|GetRotateSpeed))) false false))))

(event Custom|Apply%20Lock%20Color
  (Rendering|Material|SetVectorParameterValue (Variables|Default|GetRingColorMID) "Color" (Math|Color|Lerp(LinearColor) "(R=0.171875,G=0.171875,B=0.171875,A=1.000000)" "(R=1.000000,G=0.000000,B=0.000000,A=1.000000)" (/ (Math|Conversions|ToFloat(Integer) (Variables|Default|GetLockCount)) (Math|Conversions|ToFloat(Integer) (Variables|Default|GetMaxLockCount)))) :!class /Script/Engine.MaterialInstanceDynamic))

(event EventBeginPlay
  (bind _ring (Variables|Default|GetRing))
  (bind _returnvalue (Rendering|Material|CreateDynamicMaterialInstance _ring 0 (Rendering|Material|GetMaterial _ring 0) "None" :!class /Script/Engine.PrimitiveComponent))
  (Variables|Default|SetRingColorMID _returnvalue)
  (CallFunction|ApplyLockColor))

(event Collision|EventActorBeginOverlap
  (params (OtherActor :type Actor%20Object%20Reference))
  (bind _goalcount (Variables|Default|GetGoalCount))
  (bind _asbp_base_player (Utilities|Casting|CastToBP_BasePlayer OtherActor))
  (if (Variables|Default|GetbIsOpened)
    (Math|Integer|IncrementInt _goalcount
      (:%20%20
        (Default|Goal _asbp_base_player)
        (CallFunction|ApplyCurrentColor)
        (if (>= _goalcount 4)
          (CallFunction|StartSpinning)
          (Utilities|FlowControl|Delay 3.0)
          (CallFunction|ClearLevel))))))

(fn ConstructionScript)