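; Test player pawn for a side-scrolling level, with custom per-tick gravity, walking and jumping via swept offsets.
; The first input starts BP_TestSpawner, and every press and release is recorded in GS_TestLevelState at ticks relative to that moment.
; Unblocked horizontal moves increment the run-goal lock count.
; Holding the orb animates outline opacity and ignores orb walls; Goal and Defeat hide and disable the pawn, while SuperJump launches it upward.
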(event Custom|Set%20Ground%20State
  (bind _returnvalue (Transformation|GetActorLocation))
  (bind _returnvalue_2 (Transformation|GetActorLocation))
  (bind _returnvalue_3 (Transformation|GetActorLocation))
  (bind _outhit (Collision|LineTraceByChannel (Transformation|GetActorLocation) (Math|Vector|MakeVector (.x _returnvalue_3) (.y _returnvalue_3) (- (.z _returnvalue_3) 55.0)) "TraceTypeQuery1" false 0 "ForOneFrame"))
  (bind _result (CallFunction|IsBlocked _outhit))
  (bind _outhit_2 (Collision|LineTraceByChannel (Transformation|GetActorLocation) (Math|Vector|MakeVector (+ (.x _returnvalue) 47.0) (.y _returnvalue) (- (.z _returnvalue) 55.0)) "TraceTypeQuery1" false 0 "ForOneFrame"))
  (bind _result_2 (CallFunction|IsBlocked _outhit_2))
  (bind _outhit_3 (Collision|LineTraceByChannel (Transformation|GetActorLocation) (Math|Vector|MakeVector (- (.x _returnvalue_2) 47.0) (.y _returnvalue_2) (- (.z _returnvalue_2) 55.0)) "TraceTypeQuery1" false 0 "ForOneFrame"))
  (bind _result_3 (CallFunction|IsBlocked _outhit_3))
  (Variables|Default|SetbIsGround (Math|Boolean|ORBoolean _result _result_2 _result_3)))

(event Input|EnhancedActionEvents|EnhancedInputActionIA_TestPlayer_LeftWalk
  (params (ActionValue :type Boolean) (ElapsedSeconds :type Float%20%28double-precision%29) (TriggeredSeconds :type Float%20%28double-precision%29) (InputAction :type Input%20Action%20Object%20Reference :default "/Game/BluePrints/FrameWorks/IA_TestPlayer_LeftWalk.IA_TestPlayer_LeftWalk"))
  (:Started
    (if (Variables|Default|GetbHasMoved)
      _
      (else
        (Variables|Default|SetbHasMoved true)
        (Variables|Default|SetWorldTickThisPawnMoved (+ (Variables|/Game/BluePrints/FrameWorks/GS_TestLevelState.GS_TestLevelState_C|GetCurrentTick (Variables|Default|GetCurrentGameState)) -1))
        (Default|StartSpawn (Variables|Default|GetTargetSpawner))))
    (Variables|Default|SetKey_Left true)
    (if (Variables|Default|GetbHasMoved)
      (Default|RecordMovementInput (Variables|Default|GetCurrentGameState) "NewEnumerator0" true (- (Variables|/Game/BluePrints/FrameWorks/GS_TestLevelState.GS_TestLevelState_C|GetCurrentTick (Variables|Default|GetCurrentGameState)) (Variables|Default|GetWorldTickThisPawnMoved)))))
  (:Completed
    (Variables|Default|SetKey_Left false)
    (if (Variables|Default|GetbHasMoved)
      (Default|RecordMovementInput (Variables|Default|GetCurrentGameState) "NewEnumerator0" false (- (Variables|/Game/BluePrints/FrameWorks/GS_TestLevelState.GS_TestLevelState_C|GetCurrentTick (Variables|Default|GetCurrentGameState)) (Variables|Default|GetWorldTickThisPawnMoved))))))

(event Input|EnhancedActionEvents|EnhancedInputActionIA_TestPlayer_RightWalk
  (params (ActionValue :type Boolean) (ElapsedSeconds :type Float%20%28double-precision%29) (TriggeredSeconds :type Float%20%28double-precision%29) (InputAction :type Input%20Action%20Object%20Reference :default "/Game/BluePrints/FrameWorks/IA_TestPlayer_RightWalk.IA_TestPlayer_RightWalk"))
  (:Started
    (if (Variables|Default|GetbHasMoved)
      _
      (else
        (Variables|Default|SetbHasMoved true)
        (Variables|Default|SetWorldTickThisPawnMoved (+ (Variables|/Game/BluePrints/FrameWorks/GS_TestLevelState.GS_TestLevelState_C|GetCurrentTick (Variables|Default|GetCurrentGameState)) -1))
        (Default|StartSpawn (Variables|Default|GetTargetSpawner))))
    (Variables|Default|SetKey_Right true)
    (if (Variables|Default|GetbHasMoved)
      (Default|RecordMovementInput (Variables|Default|GetCurrentGameState) "NewEnumerator1" true (- (Variables|/Game/BluePrints/FrameWorks/GS_TestLevelState.GS_TestLevelState_C|GetCurrentTick (Variables|Default|GetCurrentGameState)) (Variables|Default|GetWorldTickThisPawnMoved)))))
  (:Completed
    (Variables|Default|SetKey_Right false)
    (if (Variables|Default|GetbHasMoved)
      (Default|RecordMovementInput (Variables|Default|GetCurrentGameState) "NewEnumerator1" false (- (Variables|/Game/BluePrints/FrameWorks/GS_TestLevelState.GS_TestLevelState_C|GetCurrentTick (Variables|Default|GetCurrentGameState)) (Variables|Default|GetWorldTickThisPawnMoved))))))

(event Input|EnhancedActionEvents|EnhancedInputActionIA_TestPlayer_Jump
  (params (ActionValue :type Boolean) (ElapsedSeconds :type Float%20%28double-precision%29) (TriggeredSeconds :type Float%20%28double-precision%29) (InputAction :type Input%20Action%20Object%20Reference :default "/Game/BluePrints/FrameWorks/IA_TestPlayer_Jump.IA_TestPlayer_Jump"))
  (:Started
    (if (Variables|Default|GetbHasMoved)
      _
      (else
        (Variables|Default|SetbHasMoved true)
        (Variables|Default|SetWorldTickThisPawnMoved (+ (Variables|/Game/BluePrints/FrameWorks/GS_TestLevelState.GS_TestLevelState_C|GetCurrentTick (Variables|Default|GetCurrentGameState)) -1))
        (Default|StartSpawn (Variables|Default|GetTargetSpawner))))
    (Variables|Default|SetKey_Jump true)
    (if (Variables|Default|GetbHasMoved)
      (Default|RecordMovementInput (Variables|Default|GetCurrentGameState) "NewEnumerator2" true (- (Variables|/Game/BluePrints/FrameWorks/GS_TestLevelState.GS_TestLevelState_C|GetCurrentTick (Variables|Default|GetCurrentGameState)) (Variables|Default|GetWorldTickThisPawnMoved)))))
  (:Completed
    (Variables|Default|SetKey_Jump false)
    (if (Variables|Default|GetbHasMoved)
      (Default|RecordMovementInput (Variables|Default|GetCurrentGameState) "NewEnumerator2" false (- (Variables|/Game/BluePrints/FrameWorks/GS_TestLevelState.GS_TestLevelState_C|GetCurrentTick (Variables|Default|GetCurrentGameState)) (Variables|Default|GetWorldTickThisPawnMoved))))))

(event EventBeginPlay
  (bind _cubeoutline (Variables|Default|GetCubeOutline))
  (Input|AddMappingContext (PlayerController|LocalPlayerSubsystems|GetEnhancedInputLocalPlayerSubsystem) "/Game/BluePrints/FrameWorks/IMC_TestPlayer.IMC_TestPlayer" 0 "(bIgnoreAllPressedKeysUntilRelease=True,bForceImmediately=False,bNotifyUserSettings=False)")
  (bind _returnvalue (Actor|GetActorOfClass "/Game/BluePrints/Actors/TestActors/BP_TestSpawner.BP_TestSpawner_C"))
  (Utilities|IsValid _returnvalue
    (:Is%20Valid
      (Variables|Default|SetTargetSpawner _returnvalue)
      (bind _asgs_test_level_state (Utilities|Casting|CastToGS_TestLevelState (Game|GetGameState)))
      (bind _output_get (Variables|Default|SetCurrentGameState _asgs_test_level_state))
      (Variables|Default|SetWorldTickThisPawnCreated (Variables|/Game/BluePrints/FrameWorks/GS_TestLevelState.GS_TestLevelState_C|GetCurrentTick _output_get))
      (bind _returnvalue_2 (Rendering|Material|CreateDynamicMaterialInstance _cubeoutline 0 (Rendering|Material|GetMaterial _cubeoutline 0) "None" :!class /Script/Engine.PrimitiveComponent))
      (Variables|Default|SetOutlineOpacityMID _returnvalue_2)
      (bind _returnvalue_3 (Actor|GetActorOfClass "/Game/BluePrints/Actors/TestActors/BP_TestRequireRunGoal.BP_TestRequireRunGoal_C"))
      (Variables|Default|SetTargetRequireRunGoal _returnvalue_3))))

(event EventMove
  (bind _targetrequirerungoal (Variables|Default|GetTargetRequireRunGoal))
  (Variables|Default|SetDirection "0, 0, 0")
  (if (Variables|Default|GetKey_Left)
    (Variables|Default|SetDirection (+ (Variables|Default|GetDirection) (Math|Vector|MakeVector -1.0 0.0 0.0))))
  (if (Variables|Default|GetKey_Right)
    (bind _output_get (Variables|Default|SetDirection (+ (Variables|Default|GetDirection) (Math|Vector|MakeVector 1.0 0.0 0.0)))))
  (bind _sweephitresult (Transformation|AddActorWorldOffset (* _output_get (Variables|Default|GetSpeed)) true))
  (if (.bBlockingHit (Collision|BreakHitResult _sweephitresult))
    _
    (else
      (Utilities|IsValid _targetrequirerungoal
        (:Is%20Valid
          (Default|IncreaseLockCount _targetrequirerungoal))
        (:Is%20Not%20Valid
          _))))
  (if (and (Variables|Default|GetKey_Jump) (Variables|Default|GetbIsGround))
    (bind _output_get_2 (Variables|Default|SetZVelocity (Variables|Default|GetJumpHeight)))
    (Transformation|AddActorWorldOffset (Math|Vector|MakeVector 0.0 0.0 (Math|Conversions|ToFloat(Integer) _output_get_2)) true)))

(event EventTick
  (params (DeltaSeconds :type Float%20%28single-precision%29))
  (bind _output_get (Variables|Default|SetZVelocity (- (Variables|Default|GetZVelocity) (Variables|Default|GetGravity))))
  (bind _sweephitresult (Transformation|AddActorWorldOffset (Math|Vector|MakeVector 0.0 0.0 (Math|Conversions|ToFloat(Integer) _output_get)) true))
  (if (.bBlockingHit (Collision|BreakHitResult _sweephitresult))
    (if (<= (Variables|Default|GetZVelocity) 0)
      (Variables|Default|SetbIsGround true)
      (else
        (Variables|Default|SetbIsGround false)))
    (Variables|Default|SetZVelocity 0)
    (else
      (Variables|Default|SetbIsGround false)))
  (CallFunction|Move))

(event EventSetHasOrb
  (Variables|Default|SetbHasOrb true)
  (bind _새_트랙_0 (Timeline|Outline%20Opacity Play)
    (:Update
      (Rendering|Material|SetScalarParameterValue (Variables|Default|GetOutlineOpacityMID) "Opacity" _새_트랙_0 :!class /Script/Engine.MaterialInstanceDynamic)
      (for _array_element (Variables|/Game/BluePrints/FrameWorks/GS_TestLevelState.GS_TestLevelState_C|GetOrbWallList (Variables|Default|GetCurrentGameState))
        (Collision|IgnoreActorwhenMoving (Variables|Default|GetBoxCollision) _array_element true)))))

(event EventGoal
  (Input|DisableInput 0)
  (Rendering|SetActorHiddenInGame true)
  (Collision|SetActorEnableCollision false)
  (Actor|Tick|SetActorTickEnabled false))

(event EventSuperJump
  (Variables|Default|SetZVelocity 50))

(event EventDefeat
  (Input|DisableInput 0)
  (Rendering|SetActorHiddenInGame true)
  (Collision|SetActorEnableCollision false)
  (Actor|Tick|SetActorTickEnabled false))

(fn ConstructionScript)

(fn IsBlocked
  (params (In%20Hit :type Hit%20Result%20Structure))
  (bind _hitactor (Collision|BreakHitResult In%20Hit))
  (Utilities|IsValid _hitactor
    (:Is%20Valid
      (if (Utilities|DoesObjectImplementInterface _hitactor "/Game/BluePrints/FrameWorks/BPI_TestForWall_CanBlock.BPI_TestForWall_CanBlock_C")
        (bind _result (Class|BPITestforWallCanBlock|CanBlock(Message) _hitactor self))
        (return _result)
        (else
          (return true))))
    (:Is%20Not%20Valid
      (return false))))

(fn GetHasOrb
  (return (Variables|Default|GetbHasOrb)))