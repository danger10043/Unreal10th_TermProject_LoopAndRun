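; BP_TestSwitchWall is a test wall actor that toggles between solid and translucent, passable states.
; BeginPlay creates a dynamic material instance on the Cube, then starts the wall disabled.
; EnableBlock and DisableBlock apply the Color and switch opacity and collision; nothing in this Blueprint calls EnableBlock.
; Both events set IsBlocking to true, so that flag does not reflect the disabled state.
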(event Custom|Enable%20Block
  (bind _cubecolormid (Variables|Default|GetCubeColorMID))
  (Rendering|Material|SetVectorParameterValue _cubecolormid "Color" (Variables|Default|GetColor) :!class /Script/Engine.MaterialInstanceDynamic)
  (Rendering|Material|SetScalarParameterValue _cubecolormid "Opacity" 1.0 :!class /Script/Engine.MaterialInstanceDynamic)
  (Collision|SetCollisionEnabled (Variables|Default|GetCube) "QueryAndPhysics")
  (Variables|Default|SetbIsBlocking true))

(event Custom|Disable%20Block
  (bind _cubecolormid (Variables|Default|GetCubeColorMID))
  (Rendering|Material|SetVectorParameterValue _cubecolormid "Color" (Variables|Default|GetColor) :!class /Script/Engine.MaterialInstanceDynamic)
  (Rendering|Material|SetScalarParameterValue _cubecolormid "Opacity" 0.35 :!class /Script/Engine.MaterialInstanceDynamic)
  (Collision|SetCollisionEnabled (Variables|Default|GetCube) "NoCollision")
  (Variables|Default|SetbIsBlocking true))

(event EventBeginPlay
  (bind _cube (Variables|Default|GetCube))
  (Variables|Default|SetbIsBlocking false)
  (bind _returnvalue (Rendering|Material|CreateDynamicMaterialInstance _cube 0 (Rendering|Material|GetMaterial _cube 0) "None" :!class /Script/Engine.PrimitiveComponent))
  (Variables|Default|SetCubeColorMID _returnvalue)
  (CallFunction|DisableBlock))

(event Collision|EventActorBeginOverlap
  (params (OtherActor :type Actor%20Object%20Reference)))

(event EventTick
  (params (DeltaSeconds :type Float%20%28single-precision%29)))

(fn ConstructionScript)