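; BP_SuperJump is a trigger actor that super-jumps any BP_BasePlayer overlapping it, much like a jump pad.
; Begin and end overlap events add and remove players from the InActorList set.
; Every Tick calls SuperJump on each tracked player with a fixed value and spawns the NS_Heal_Cast Niagara effect at their location, so both repeat each frame during overlap.
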(event EventBeginPlay)

(event EventTick
  (params (DeltaSeconds :type Float%20%28single-precision%29))
  (bind _valuepin (Utilities|Set|ForEachLoop(Set) (Variables|Default|GetInActorList))
    (:then
      (Default|SuperJump _valuepin 50)
      (Niagara|SpawnSystematLocation "/Game/ExternalAsset/Vefects/Anime_Stylized_VFX/VFX/Particles/NS_Heal_Cast.NS_Heal_Cast" (Transformation|GetActorLocation _valuepin)))))

(event Collision|EventActorBeginOverlap
  (params (OtherActor :type Actor%20Object%20Reference))
  (bind _asbp_base_player (Utilities|Casting|CastToBP_BasePlayer OtherActor))
  (Utilities|Set|Add (Variables|Default|GetInActorList) _asbp_base_player))

(event Collision|EventActorEndOverlap
  (params (OtherActor :type Actor%20Object%20Reference))
  (bind _asbp_base_player (Utilities|Casting|CastToBP_BasePlayer OtherActor))
  (Utilities|Set|Remove (Variables|Default|GetInActorList) _asbp_base_player))

(fn ConstructionScript)