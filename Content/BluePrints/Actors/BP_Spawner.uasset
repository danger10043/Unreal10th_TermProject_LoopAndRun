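; BP_Spawner is a spawn station that creates player copies, either stable or unstable, and can move the player to its spawn point on BeginPlay.
; BeginPlay also caches the progress bar widget and picks the spawn effect, tinting the bar red for unstable copies.
; StartSpawn plays a timeline that fills the bar, then on its event track spawns BP_PlayerCopy with the effect if Spawnable, marking it unstable when flagged.
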(event Custom|Start%20Spawn
  (bind _spawnpoint (Variables|Default|GetSpawnPoint))
  (bind _returnvalue (Transformation|GetWorldTransform _spawnpoint))
  (bind (_location _rotation) (Math|Transform|BreakTransform _returnvalue))
  (bind _coloralpha (Timeline|타임라인 Play)
    (:Update
      (Default|SetPercent (Variables|Default|GetProgressBarUI) _coloralpha))
    (:Event%20Trigger
      (if (Variables|Default|GetbSpawnable)
        (bind _returnvalue_2 (Game|SpawnActorfromClass "/Game/BluePrints/Actors/BP_PlayerCopy.BP_PlayerCopy_C" _returnvalue "Undefined" "MultiplyWithRoot" 0 0))
        (Niagara|SpawnSystematLocation (Variables|Default|GetSpawnEffect) _location _rotation "2.000000,2.000000,2.000000")
        (if (Variables|Default|GetbDoSpawnUnstableCopy)
          (Default|SetUnstable _returnvalue_2))))))

(event EventBeginPlay
  (bind _aswbp_spawner_progress_bar (Utilities|Casting|CastToWBP_SpawnerProgressBar (UserInterface|GetWidget (Variables|Default|GetProgressBar))))
  (Variables|Default|SetProgressBarUI _aswbp_spawner_progress_bar)
  (if (Variables|Default|GetbDoTeleportPlayerToSpawner)
    (Transformation|SetActorLocation (Game|Player|GetPlayerPawn 0) (Transformation|GetWorldLocation (Variables|Default|GetSpawnPoint)) false false))
  (if (Variables|Default|GetbDoSpawnUnstableCopy)
    (Variables|Default|SetSpawnEffect (Variables|Default|GetSpawnEffectUnstable))
    (Class|WidgetComponent|SetTintColorandOpacity (Variables|Default|GetProgressBar) "(R=1.000000,G=0.000000,B=0.000000,A=1.000000)")
    (else
      (Variables|Default|SetSpawnEffect (Variables|Default|GetSpawnEffectStable)))))

(fn ConstructionScript)