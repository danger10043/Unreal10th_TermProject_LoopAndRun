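; BP_Goal is the level's goal portal, which counts arriving players and clears the level at four.
; In lock mode it disables the portal and tracks overlapping players until IncreaseLockCount reaches the maximum, then EnableGoal opens it and sends those players through.
; Progress changes feed a buffer that Tick eases into the widget bar.
; A full bar with enough goals triggers win VFX, then the clear UI and disabled input.
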(event Custom|Debug%20Event)

(event Custom|Clear
  (bind _returnvalue (Game|GetPlayerController 0))
  (UserInterface|Viewport|AddtoViewport (Variables|/Game/BluePrints/FrameWorks/GS_LevelState.GS_LevelState_C|GetClearUI (Variables|Default|GetGameState)) 0)
  (Variables|/Script/Engine.PlayerController|SetbShowMouseCursor _returnvalue true)
  (Input|DisableInput (Game|Player|GetPlayerPawn 0) _returnvalue))

(event EventBeginPlay
  (bind _aswbp_goal_progress_bar (Utilities|Casting|CastToWBP_GoalProgressBar (UserInterface|GetWidget (Variables|Default|GetProgressBar))))
  (bind _output_get (Variables|Default|SetProgressBarUI _aswbp_goal_progress_bar))
  (Default|SetPercent _output_get 0.0)
  (bind _asgs_level_state (Utilities|Casting|CastToGS_LevelState (Game|GetGameState)))
  (Variables|Default|SetGameState _asgs_level_state)
  (if (Variables|Default|GetbIsLockMode)
    (Class|WidgetComponent|SetTintColorandOpacity (Variables|Default|GetProgressBar) "(R=1.000000,G=0.000000,B=0.000000,A=1.000000)")
    (bind _asbp_goal_mesh (Utilities|Casting|CastToBP_GoalMesh (Variables|/Script/Engine.ChildActorComponent|GetChildActor (Variables|Default|GetPortalMesh))))
    (Default|DisablePortal _asbp_goal_mesh)))

(event Collision|EventActorBeginOverlap
  (params (OtherActor :type Actor%20Object%20Reference))
  (bind _asbp_base_player (Utilities|Casting|CastToBP_BasePlayer OtherActor))
  (if (not (Variables|Default|GetbIsLockMode))
    (Math|Integer|IncrementInt (Variables|Default|GetGoalCount)
      (:%20%20
        (Default|Goal _asbp_base_player)
        (CallFunction|AddProgressPercent 0.25)))
    (else
      (Utilities|Set|Add (Variables|Default|GetCurrentInPlayerList) _asbp_base_player))))

(event EventTick
  (params (DeltaSeconds :type Float%20%28single-precision%29))
  (if (> (Math|Float|Absolute(Float) (Variables|Default|GetProgressBarValueBuffer)) 0.0)
    (CallFunction|ConsumeBuffer 0.05)
    (if (and (>= (Variables|Default|GetGoalCount) 4) (> (Variables|Default|GetCurrentProgressBarValue) 0.97))
      (Utilities|FlowControl|DoOnce false
        (:Completed
          (Niagara|SpawnSystematLocation "/Game/BluePrints/VFX/NS_GoalWinGame.NS_GoalWinGame" (Transformation|GetWorldLocation (Variables|Default|GetNiagaraPoint)) "0, 0, 0" "1.500000,1.500000,1.500000")
          (Utilities|FlowControl|Delay 1.2)
          (Class|WidgetComponent|SetTintColorandOpacity (Variables|Default|GetProgressBar) "(R=0.000000,G=0.800000,B=1.000000,A=1.000000)")
          (Utilities|FlowControl|Delay 2.0)
          (CallFunction|Clear))))))

(event Collision|EventActorEndOverlap
  (params (OtherActor :type Actor%20Object%20Reference))
  (bind _asbp_base_player (Utilities|Casting|CastToBP_BasePlayer OtherActor))
  (if (Variables|Default|GetbIsLockMode)
    (Utilities|Set|Remove (Variables|Default|GetCurrentInPlayerList) _asbp_base_player)))

(fn ConstructionScript)

(fn ConsumeBuffer
  (params (Speed :type Float%20%28double-precision%29))
  (if (<= (Math|Float|Absolute(Float) (Variables|Default|GetProgressBarValueBuffer)) 0.003)
    (Variables|Default|SetCurrentProgressBarValue (Math|Float|Clamp(Float) (+ (Variables|Default|GetCurrentProgressBarValue) (Variables|Default|GetProgressBarValueBuffer))))
    (Variables|Default|SetProgressBarValueBuffer 0.0)
    (else
      (Variables|Default|SetCurrentProgressBarValue (Math|Float|Clamp(Float) (+ (* (Variables|Default|GetProgressBarValueBuffer) Speed) (Variables|Default|GetCurrentProgressBarValue))))
      (Variables|Default|SetProgressBarValueBuffer (* (Variables|Default|GetProgressBarValueBuffer) (- 1.0 Speed)))))
  (Default|SetPercent (Variables|Default|GetProgressBarUI) (Variables|Default|GetCurrentProgressBarValue)))

(fn SetProgressPercent
  (params (In%20Percent :type Float%20%28double-precision%29))
  (Variables|Default|SetProgressBarValueBuffer (+ (- In%20Percent (Variables|Default|GetCurrentProgressBarValue)) (Variables|Default|GetProgressBarValueBuffer)))
  (return))

(fn AddProgressPercent
  (params (In%20Percent :type Float%20%28double-precision%29))
  (Variables|Default|SetProgressBarValueBuffer (+ In%20Percent (Variables|Default|GetProgressBarValueBuffer))))

(fn IncreaseLockCount
  (bind _lockcount (Variables|Default|GetLockCount))
  (bind _maxlockcount (Variables|Default|GetMaxLockCount))
  (bind _returnvalue (Math|Conversions|ToFloat(Integer) _lockcount))
  (bind _returnvalue_2 (Math|Conversions|ToFloat(Integer) _maxlockcount))
  (bind _returnvalue_3 (/ _returnvalue _returnvalue_2))
  (if (Variables|Default|GetbIsLockMode)
    (bind _result (Math|Integer|IncrementInt (Variables|Default|GetLockCount))
      (:%20%20
        (if (>= _result (Variables|Default|GetMaxLockCount))
          (CallFunction|EnableGoal)
          (return)
          (else
            (Default|SetPercent (Variables|Default|GetProgressBarUI) _returnvalue_3)
            (Variables|Default|SetCurrentProgressBarValue _returnvalue_3)))))
    (else
      (return))))

(fn EnableGoal
  (Variables|Default|SetbIsLockMode false)
  (CallFunction|SetProgressPercent 0.0)
  (Class|WidgetComponent|SetTintColorandOpacity (Variables|Default|GetProgressBar) "(R=0.700000,G=0.200000,B=0.000000,A=1.000000)")
  (bind _asbp_goal_mesh (Utilities|Casting|CastToBP_GoalMesh (Variables|/Script/Engine.ChildActorComponent|GetChildActor (Variables|Default|GetPortalMesh))))
  (Default|EnablePortal _asbp_goal_mesh)
  (Niagara|SpawnSystematLocation "/Game/BluePrints/VFX/NS_GoalEnablePortal.NS_GoalEnablePortal" (Transformation|GetWorldLocation (Variables|Default|GetNiagaraPoint)))
  (bind _valuepin (Utilities|Set|ForEachLoop(Set) (Variables|Default|GetCurrentInPlayerList))
    (:then
      (Default|Goal _valuepin)
      (CallFunction|AddProgressPercent 0.25))))