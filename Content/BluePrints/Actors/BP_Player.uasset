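; BP_Player is the player pawn: it walks left or right, jumps, and is hidden and disabled with an effect on reaching the goal.
; The first input starts BP_Spawner and enables gravity; every press and release is recorded in the GameState with a tick relative to that moment.
; TickOverride applies swept movement from key flags, can raise BP_Goal's lock count when unblocked, and turns the cursor toward BP_Camera.
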(event Input|EnhancedActionEvents|EnhancedInputActionIA_TestPlayer_LeftWalk
  (params (ActionValue :type Boolean) (ElapsedSeconds :type Float%20%28double-precision%29) (TriggeredSeconds :type Float%20%28double-precision%29) (InputAction :type Input%20Action%20Object%20Reference :default "/Game/BluePrints/FrameWorks/IA_TestPlayer_LeftWalk.IA_TestPlayer_LeftWalk"))
  ;[0.15 0.15 0.15 0.5] 좌, 우, 점프 입력 받기. 입력 후 이동 및 입력 기록 GameState에 저장
  (:Started
    (if (Variables|Default|GetbHasMoved)
      _
      (else
        (Variables|Default|SetbHasMoved true)
        (Variables|Default|SetWorldTickThisPawnMoved (+ (Variables|/Game/BluePrints/FrameWorks/GS_LevelState.GS_LevelState_C|GetCurrentTick (Variables|Default|GetCurrentGameState)) -1))
        (Default|StartSpawn (Variables|Default|GetTestSpawner))))
    (Variables|Default|SetKey_Left true)
    (if (Variables|Default|GetbHasMoved)
      (Default|RecordMovementInput (Variables|Default|GetCurrentGameState) "NewEnumerator0" true (- (Variables|/Game/BluePrints/FrameWorks/GS_LevelState.GS_LevelState_C|GetCurrentTick (Variables|Default|GetCurrentGameState)) (Variables|Default|GetWorldTickThisPawnMoved)))))
  (:Completed
    (Variables|Default|SetKey_Left false)
    (if (Variables|Default|GetbHasMoved)
      (Default|RecordMovementInput (Variables|Default|GetCurrentGameState) "NewEnumerator0" false (- (Variables|/Game/BluePrints/FrameWorks/GS_LevelState.GS_LevelState_C|GetCurrentTick (Variables|Default|GetCurrentGameState)) (Variables|Default|GetWorldTickThisPawnMoved))))))

(event Input|EnhancedActionEvents|EnhancedInputActionIA_TestPlayer_RightWalk
  (params (ActionValue :type Boolean) (ElapsedSeconds :type Float%20%28double-precision%29) (TriggeredSeconds :type Float%20%28double-precision%29) (InputAction :type Input%20Action%20Object%20Reference :default "/Game/BluePrints/FrameWorks/IA_TestPlayer_RightWalk.IA_TestPlayer_RightWalk"))
  ;[0.15 0.15 0.15 0.5] 좌, 우, 점프 입력 받기. 입력 후 이동 및 입력 기록 GameState에 저장
  (:Started
    (if (Variables|Default|GetbHasMoved)
      _
      (else
        (Variables|Default|SetbHasMoved true)
        (Variables|Default|SetWorldTickThisPawnMoved (+ (Variables|/Game/BluePrints/FrameWorks/GS_LevelState.GS_LevelState_C|GetCurrentTick (Variables|Default|GetCurrentGameState)) -1))
        (Default|StartSpawn (Variables|Default|GetTestSpawner))))
    (Variables|Default|SetKey_Right true)
    (if (Variables|Default|GetbHasMoved)
      (Default|RecordMovementInput (Variables|Default|GetCurrentGameState) "NewEnumerator1" true (- (Variables|/Game/BluePrints/FrameWorks/GS_LevelState.GS_LevelState_C|GetCurrentTick (Variables|Default|GetCurrentGameState)) (Variables|Default|GetWorldTickThisPawnMoved)))))
  (:Completed
    (Variables|Default|SetKey_Right false)
    (if (Variables|Default|GetbHasMoved)
      (Default|RecordMovementInput (Variables|Default|GetCurrentGameState) "NewEnumerator1" false (- (Variables|/Game/BluePrints/FrameWorks/GS_LevelState.GS_LevelState_C|GetCurrentTick (Variables|Default|GetCurrentGameState)) (Variables|Default|GetWorldTickThisPawnMoved))))))

(event Input|EnhancedActionEvents|EnhancedInputActionIA_TestPlayer_Jump
  (params (ActionValue :type Boolean) (ElapsedSeconds :type Float%20%28double-precision%29) (TriggeredSeconds :type Float%20%28double-precision%29) (InputAction :type Input%20Action%20Object%20Reference :default "/Game/BluePrints/FrameWorks/IA_TestPlayer_Jump.IA_TestPlayer_Jump"))
  ;[0.15 0.15 0.15 0.5] 좌, 우, 점프 입력 받기. 입력 후 이동 및 입력 기록 GameState에 저장
  (:Started
    (if (Variables|Default|GetbHasMoved)
      _
      (else
        (Variables|Default|SetbHasMoved true)
        (Variables|Default|SetWorldTickThisPawnMoved (+ (Variables|/Game/BluePrints/FrameWorks/GS_LevelState.GS_LevelState_C|GetCurrentTick (Variables|Default|GetCurrentGameState)) -1))
        (Default|StartSpawn (Variables|Default|GetTestSpawner))))
    (Variables|Default|SetKey_Jump true)
    (if (Variables|Default|GetbHasMoved)
      (Default|RecordMovementInput (Variables|Default|GetCurrentGameState) "NewEnumerator2" true (- (Variables|/Game/BluePrints/FrameWorks/GS_LevelState.GS_LevelState_C|GetCurrentTick (Variables|Default|GetCurrentGameState)) (Variables|Default|GetWorldTickThisPawnMoved)))))
  (:Completed
    (Variables|Default|SetKey_Jump false)
    (if (Variables|Default|GetbHasMoved)
      (Default|RecordMovementInput (Variables|Default|GetCurrentGameState) "NewEnumerator2" false (- (Variables|/Game/BluePrints/FrameWorks/GS_LevelState.GS_LevelState_C|GetCurrentTick (Variables|Default|GetCurrentGameState)) (Variables|Default|GetWorldTickThisPawnMoved))))))

(fn ConstructionScript
  (|CallParentFunction))

(fn Initialize
  (Input|AddMappingContext (PlayerController|LocalPlayerSubsystems|GetEnhancedInputLocalPlayerSubsystem) "/Game/BluePrints/FrameWorks/IMC_TestPlayer.IMC_TestPlayer" 0 "(bIgnoreAllPressedKeysUntilRelease=True,bForceImmediately=False,bNotifyUserSettings=False)")
  (bind _returnvalue (Actor|GetActorOfClass "/Game/BluePrints/Actors/BP_Spawner.BP_Spawner_C"))
  (Utilities|IsValid _returnvalue
    (:Is%20Valid
      (Variables|Default|SetTestSpawner _returnvalue))
    (:Is%20Not%20Valid
      _))
  (bind _returnvalue_2 (Actor|GetActorOfClass "/Game/BluePrints/Actors/BP_Goal.BP_Goal_C"))
  (Variables|Default|SetTargetGoal _returnvalue_2)
  (bind _returnvalue_3 (Actor|GetActorOfClass "/Game/BluePrints/Actors/BP_Camera.BP_Camera_C"))
  (Utilities|IsValid _returnvalue_3
    (:Is%20Valid
      (Variables|Default|SetTargetCamera _returnvalue_3))
    (:Is%20Not%20Valid
      _))
  (|CallParentFunction))

(fn Move
  (Variables|Default|SetDirection "0, 0, 0")
  (if (Variables|Default|GetKey_Left)
    (Variables|Default|SetDirection (+ (Variables|Default|GetDirection) (Math|Vector|MakeVector -1.0 0.0 0.0))))
  (if (Variables|Default|GetKey_Right)
    (bind _output_get (Variables|Default|SetDirection (+ (Variables|Default|GetDirection) (Math|Vector|MakeVector 1.0 0.0 0.0)))))
  (bind _sweephitresult (Transformation|AddActorWorldOffset (* _output_get (Variables|Default|GetSpeed)) true))
  (if (.bBlockingHit (Collision|BreakHitResult _sweephitresult))
    _
    (elif (> (Math|Vector|VectorLengthXY (Variables|Default|GetCurrentVelocity)) 0.0)
      (Default|IncreaseLockCount (Variables|Default|GetTargetGoal))))
  (if (and (Variables|Default|GetKey_Jump) (Variables|Default|GetbIsGround))
    (bind _output_get_2 (Variables|Default|SetZVelocity (Variables|Default|GetJumpHeight)))
    (Transformation|AddActorWorldOffset (Math|Vector|MakeVector 0.0 0.0 (Math|Conversions|ToFloat(Integer) _output_get_2)) true)
    (|CallParentFunction)))

(fn Goal
  (bind _returnvalue (Transformation|GetActorLocation))
  (Niagara|SpawnSystematLocation "/Game/BluePrints/VFX/NS_PlayerGoal.NS_PlayerGoal" (Math|Vector|MakeVector (.x _returnvalue) (.y _returnvalue) (- (.z _returnvalue) 4e+01)) "0, 0, 0" "0.500000,0.500000,1.000000")
  (Input|DisableInput 0)
  (Rendering|SetActorHiddenInGame true)
  (Collision|SetActorEnableCollision false)
  (Actor|Tick|SetActorTickEnabled false)
  (|CallParentFunction))

(fn TickOverride
  (CallFunction|Move)
  (CallFunction|RotateUI)
  (|CallParentFunction))

(fn RotateUI
  (bind _playercursor (Variables|Default|GetPlayerCursor))
  (Transformation|SetWorldRotation _playercursor (Math|Rotator|MakeRotfromX (Math|Vector|Normalize (- (Transformation|GetActorLocation (Variables|Default|GetTargetCamera)) (Transformation|GetWorldLocation _playercursor)))) false false)
  (return))

(fn ApplyGravity
  (if (Variables|Default|GetbHasMoved)
    (|CallParentFunction)))