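; Player copy actor for the test level that replays recorded left, right and jump inputs from GS_TestLevelState, timed from its spawn tick.
; Each Tick applies gravity through swept offsets, sets grounding from the vertical hit, consumes at most one due input, then moves.
; SetHasOrb animates outline opacity and makes the collision box ignore orb walls while moving.
; SuperJump boosts vertical velocity, while Goal and Defeat hide and disable the copy.
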(event Custom|Apply%20State
  (bind _currentinputdatalistindex (Variables|Default|GetCurrentInputDataListIndex))
  (bind _currentgamestate (Variables|Default|GetCurrentGameState))
  (bind _inputdatalist (Variables|/Game/BluePrints/FrameWorks/GS_TestLevelState.GS_TestLevelState_C|GetInputDataList _currentgamestate))
  (bind _output (Utilities|Array|Get(acopy) _inputdatalist _currentinputdatalistindex))
  (bind (_inputdata _ispressed _executetick) (Utilities|Struct|BreakF_InputData _output))
  (if (< (Variables|Default|GetCurrentInputDataListIndex) (Utilities|Array|Length _inputdatalist))
    (if (>= (- (Variables|/Game/BluePrints/FrameWorks/GS_TestLevelState.GS_TestLevelState_C|GetCurrentTick (Variables|Default|GetCurrentGameState)) (Variables|Default|GetWorldTickThisPawnCreated)) _executetick)
      (switch Utilities|FlowControl|Switch|SwitchonE_InputDataEnum _inputdata
        (:NewEnumerator0
          (Variables|Default|SetKey_Left _ispressed))
        (:NewEnumerator1
          (Variables|Default|SetKey_Right _ispressed))
        (:NewEnumerator2
          (Variables|Default|SetKey_Jump _ispressed)))
      (Math|Integer|IncrementInt (Variables|Default|GetCurrentInputDataListIndex)))))

(event Custom|Set%20Ground%20State
  (bind _returnvalue (Transformation|GetActorLocation))
  (bind _returnvalue_2 (Transformation|GetActorLocation))
  (bind _returnvalue_3 (Transformation|GetActorLocation))
  (bind _outhit (Collision|LineTraceByChannel (Transformation|GetActorLocation) (Math|Vector|MakeVector (.x _returnvalue_3) (.y _returnvalue_3) (- (.z _returnvalue_3) 55.0)) "TraceTypeQuery1" false 0 "ForOneFrame"))
  (bind _result (CallFunction|IsBlocked _outhit))
  (bind _outhit_2 (Collision|LineTraceByChannel (Transformation|GetActorLocation) (Math|Vector|MakeVector (+ (.x _returnvalue) 47.0) (.y _returnvalue) (- (.z _returnvalue) 55.0)) "TraceTypeQuery1" false 0 "ForOneFrame"))
  (bind _result_2 (CallFunction|IsBlocked _outhit_2))
  (bind _outhit_3 (Collision|LineTraceByChannel (Transformation|GetActorLocation) (Math|Vector|MakeVector (- (.x _returnvalue_2) 47.0) (.y _returnvalue_2) (- (.z _returnvalue_2) 55.0)) "TraceTypeQuery1" false 0 "ForOneFrame"))
  (bind _result_3 (CallFunction|IsBlocked _outhit_3))
  (Variables|Default|SetbIsGround (Math|Boolean|ORBoolean _result _result_2 _result_3)))

(event EventBeginPlay
  (bind _cubeoutline (Variables|Default|GetCubeOutline))
  (bind _asbp_test_player (Utilities|Casting|CastToBP_TestPlayer (Game|Player|GetPlayerPawn 0)))
  (Variables|Default|SetPlayerPawn _asbp_test_player)
  (bind _asgs_test_level_state (Utilities|Casting|CastToGS_TestLevelState (Game|GetGameState)))
  (bind _output_get (Variables|Default|SetCurrentGameState _asgs_test_level_state))
  (Variables|Default|SetWorldTickThisPawnCreated (Variables|/Game/BluePrints/FrameWorks/GS_TestLevelState.GS_TestLevelState_C|GetCurrentTick _output_get))
  (bind _returnvalue (Rendering|Material|CreateDynamicMaterialInstance _cubeoutline 0 (Rendering|Material|GetMaterial _cubeoutline 0) "None" :!class /Script/Engine.PrimitiveComponent))
  (Variables|Default|SetOutlineOpacityMID _returnvalue))

(event EventMove
  (Variables|Default|SetDirection "0, 0, 0")
  (if (Variables|Default|GetKey_Left)
    (Variables|Default|SetDirection (+ (Variables|Default|GetDirection) (Math|Vector|MakeVector -1.0 0.0 0.0))))
  (if (Variables|Default|GetKey_Right)
    (bind _output_get (Variables|Default|SetDirection (+ (Variables|Default|GetDirection) (Math|Vector|MakeVector 1.0 0.0 0.0)))))
  (Transformation|AddActorWorldOffset (* _output_get (Variables|Default|GetSpeed)) true)
  (if (and (Variables|Default|GetKey_Jump) (Variables|Default|GetbIsGround))
    (bind _output_get_2 (Variables|Default|SetZVelocity (Variables|Default|GetJumpHeight)))
    (Transformation|AddActorWorldOffset (Math|Vector|MakeVector 0.0 0.0 (Math|Conversions|ToFloat(Integer) _output_get_2)) true)))

(event EventTick
  (params (DeltaSeconds :type Float%20%28single-precision%29))
  (bind _output_get (Variables|Default|SetZVelocity (- (Variables|Default|GetZVelocity) (Variables|Default|GetGravity))))
  (bind _sweephitresult (Transformation|AddActorWorldOffset (Math|Vector|MakeVector 0.0 0.0 (Math|Conversions|ToFloat(Integer) _output_get)) true))
  (if (.bBlockingHit (Collision|BreakHitResult _sweephitresult))
    (if (<= (Variables|Default|GetZVelocity) 0)
      (Variables|Default|SetbIsGround true)
      (else
        (Variables|Default|SetbIsGround false)))
    (Variables|Default|SetZVelocity 0)
    (else
      (Variables|Default|SetbIsGround false)))
  (CallFunction|ApplyState)
  (CallFunction|Move))

(event EventSetHasOrb
  (Variables|Default|SetbHasOrb true)
  (bind _새_트랙_0 (Timeline|타임라인 Play)
    (:Update
      (Rendering|Material|SetScalarParameterValue (Variables|Default|GetOutlineOpacityMID) "Opacity" _새_트랙_0 :!class /Script/Engine.MaterialInstanceDynamic)
      (for _array_element (Variables|/Game/BluePrints/FrameWorks/GS_TestLevelState.GS_TestLevelState_C|GetOrbWallList (Variables|Default|GetCurrentGameState))
        (Collision|IgnoreActorwhenMoving (Variables|Default|GetBoxCollision) _array_element true)))))

(event EventGoal
  (Rendering|SetActorHiddenInGame true)
  (Collision|SetActorEnableCollision false)
  (Actor|Tick|SetActorTickEnabled false))

(event EventSuperJump
  (Variables|Default|SetZVelocity 50))

(event EventDefeat
  (Rendering|SetActorHiddenInGame true)
  (Collision|SetActorEnableCollision false)
  (Actor|Tick|SetActorTickEnabled false))

(fn ConstructionScript)

(fn IsBlocked
  (params (In%20Hit :type Hit%20Result%20Structure))
  (bind _hitactor (Collision|BreakHitResult In%20Hit))
  (Utilities|IsValid _hitactor
    (:Is%20Valid
      (if (Utilities|DoesObjectImplementInterface _hitactor "/Game/BluePrints/FrameWorks/BPI_TestForWall_CanBlock.BPI_TestForWall_CanBlock_C")
        (bind _result (Class|BPITestforWallCanBlock|CanBlock(Message) _hitactor self))
        (return _result)
        (else
          (return true))))
    (:Is%20Not%20Valid
      (return false))))

(fn GetHasOrb
  (return (Variables|Default|GetbHasOrb)))