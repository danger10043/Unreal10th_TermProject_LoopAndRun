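; BP_TestSuperJump is a test actor that sends a super jump message to eligible actors overlapping it.
; Begin overlap adds actors implementing the BPI_TestSuperJump interface to the InActorList set, and end overlap removes them.
; Every Tick it loops over that set and calls SuperJumpMessage on each member, so the message repeats for as long as the overlap lasts.
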(event EventBeginPlay)

(event EventTick
  (params (DeltaSeconds :type Float%20%28single-precision%29))
  (bind _valuepin (Utilities|Set|ForEachLoop(Set) (Variables|Default|GetInActorList))
    (:then
      (Class|BPITestSuperJump|SuperJump(Message) _valuepin))))

(event Collision|EventActorBeginOverlap
  (params (OtherActor :type Actor%20Object%20Reference))
  (if (Utilities|DoesObjectImplementInterface OtherActor "/Game/BluePrints/FrameWorks/BPI_TestSuperJump.BPI_TestSuperJump_C")
    (Utilities|Set|Add (Variables|Default|GetInActorList) OtherActor)))

(event Collision|EventActorEndOverlap
  (params (OtherActor :type Actor%20Object%20Reference))
  (Utilities|Set|Remove (Variables|Default|GetInActorList) OtherActor))

(fn ConstructionScript)