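; GS_LevelState is the level state Blueprint that tracks tick-stamped movement input and drives the tutorial pages.
; BeginPlay caches the player pawn and all orb walls and creates the tutorial widget.
; A per-frame tick counter runs alongside an event that logs movement presses and releases with a supplied execution tick.
; Page changes swap the image and navigation buttons, show the cursor and disable pawn input until GameStart restores it.
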(event Custom|Record%20Movement%20Input
  (params (Movement%20Type :type E_InputDataEnum%20Enum :default "NewEnumerator0") (Is%20Pressed :type Boolean) (Execute%20Tick :type Integer))
  (Utilities|Array|Add (Variables|Default|GetInputDataList) (Utilities|Struct|MakeF_InputData Movement%20Type Is%20Pressed Execute%20Tick)))

(event Custom|Show%20Tutorial%20Next%20Page
  (Math|Integer|IncrementInt (Variables|Default|GetCurrentTutorialPage)
    (:%20%20
      (CallFunction|RefreshPage))))

(event Custom|RefreshPage
  (bind _returnvalue (Game|GetPlayerController 0))
  (bind _tutorialui (Variables|Default|GetTutorialUI))
  (bind _tutorialui_2 (Variables|Default|GetTutorialUI))
  (Appearance|SetBrushfromTexture (Variables|/Game/BluePrints/UI/WBP_TutorialUI.WBP_TutorialUI_C|GetTutorialImage (Variables|Default|GetTutorialUI)) (Utilities|Array|Get(acopy) (Variables|Default|GetTutorialImageSet) (Variables|Default|GetCurrentTutorialPage)) false)
  (if (== (Variables|Default|GetCurrentTutorialPage) (- (Utilities|Array|Length (Variables|Default|GetTutorialImageSet)) 1))
    (Variables|/Script/UMG.Widget|SetVisibility (Variables|/Game/BluePrints/UI/WBP_TutorialUI.WBP_TutorialUI_C|GetNextButton _tutorialui) "Collapsed")
    (Variables|/Script/UMG.Widget|SetVisibility (Variables|/Game/BluePrints/UI/WBP_TutorialUI.WBP_TutorialUI_C|GetStartButton _tutorialui) "Visible")
    (else
      (Variables|/Script/UMG.Widget|SetVisibility (Variables|/Game/BluePrints/UI/WBP_TutorialUI.WBP_TutorialUI_C|GetNextButton _tutorialui_2) "Visible")
      (Variables|/Script/UMG.Widget|SetVisibility (Variables|/Game/BluePrints/UI/WBP_TutorialUI.WBP_TutorialUI_C|GetStartButton _tutorialui_2) "Collapsed")))
  (if (== (Variables|Default|GetCurrentTutorialPage) 0)
    (Variables|/Script/UMG.Widget|SetVisibility (Variables|/Game/BluePrints/UI/WBP_TutorialUI.WBP_TutorialUI_C|GetPrevButton (Variables|Default|GetTutorialUI)) "Collapsed")
    (else
      (Variables|/Script/UMG.Widget|SetVisibility (Variables|/Game/BluePrints/UI/WBP_TutorialUI.WBP_TutorialUI_C|GetPrevButton (Variables|Default|GetTutorialUI)) "Visible")))
  (Variables|/Script/Engine.PlayerController|SetbShowMouseCursor _returnvalue true)
  (Input|DisableInput (Game|Player|GetPlayerPawn 0) _returnvalue))

(event Custom|Show%20Tutorial%20Prev%20Page
  (Math|Integer|DecrementInt (Variables|Default|GetCurrentTutorialPage)
    (:%20%20
      (CallFunction|RefreshPage))))

(event Custom|GameStart
  (Input|EnableInput (Game|Player|GetPlayerPawn 0) (Game|GetPlayerController 0)))

(event EventBeginPlay
  (bind _asbp_player (Utilities|Casting|CastToBP_Player (Game|Player|GetPlayerPawn 0)))
  (Variables|Default|SetPlayerPawn _asbp_player)
  (bind _outactors (Actor|GetAllActorsOfClass "/Game/BluePrints/Actors/BP_OrbWall.BP_OrbWall_C"))
  (Variables|Default|SetOrbWallList _outactors)
  (bind _returnvalue (UserInterface|CreateWidget "/Game/BluePrints/UI/WBP_TutorialUI.WBP_TutorialUI_C" (Game|GetPlayerController 0)))
  (Variables|Default|SetTutorialUI _returnvalue))

(event EventTick
  (params (DeltaSeconds :type Float%20%28single-precision%29))
  (Math|Integer|IncrementInt (Variables|Default|GetCurrentTick)))

(fn ConstructionScript)