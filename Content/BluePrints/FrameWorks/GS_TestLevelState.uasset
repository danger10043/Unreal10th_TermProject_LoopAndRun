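; GS_TestLevelState is the test level's state Blueprint, which keeps a tick counter and a log of movement inputs.
; On BeginPlay it caches the first player pawn as BP_Player and, if that cast succeeds, gathers every BP_OrbWall in the level.
; Tick increments CurrentTick once per frame.
; RecordMovementInput appends the movement type, pressed state and a caller-supplied execute tick to InputDataList as FInputData entries.
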(event Custom|Record%20Movement%20Input
  (params (Movement%20Type :type E_InputDataEnum%20Enum :default "NewEnumerator0") (Is%20Pressed :type Boolean) (Execute%20Tick :type Integer))
  (Utilities|Array|Add (Variables|Default|GetInputDataList) (Utilities|Struct|MakeF_InputData Movement%20Type Is%20Pressed Execute%20Tick)))

(event EventBeginPlay
  (bind _asbp_player (Utilities|Casting|CastToBP_Player (Game|Player|GetPlayerPawn 0)))
  (Variables|Default|SetPlayerPawn _asbp_player)
  (bind _outactors (Actor|GetAllActorsOfClass "/Game/BluePrints/Actors/BP_OrbWall.BP_OrbWall_C"))
  (Variables|Default|SetOrbWallList _outactors))

(event EventTick
  (params (DeltaSeconds :type Float%20%28single-precision%29))
  (Math|Integer|IncrementInt (Variables|Default|GetCurrentTick)))

(fn ConstructionScript)